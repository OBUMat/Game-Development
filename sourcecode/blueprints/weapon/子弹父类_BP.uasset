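; Base bullet projectile Blueprint that plays the weapon sound on spawn and resolves impacts against zombies and the world.
; Zombie hits spawn blood and smoke, play a flesh sound and apply higher damage on the head bone.
; Other hits leave a temporary decal and use a small sphere trace to pick surface-specific particles and sound.
; Every hit pushes physics-simulating components with a velocity-based impulse, then destroys the bullet.
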(event `self.ReceiveBeginPlay`
  (`GameplayStatics.PlaySoundAtLocation` (`self.武器音效`) (`self.K2_GetActorLocation`) (struct) 1.0 1.0 0.0 null null null))

(event `self.ReceiveHit`
  (params (MyComp :type "PrimitiveComponent Object Reference") (Other :type "Actor Object Reference") (OtherComp :type "PrimitiveComponent Object Reference") (bSelfMoved :type Boolean) (HitLocation :type "Vector Structure") (HitNormal :type "Vector Structure") (NormalImpulse :type "Vector Structure") (Hit :type "HitResult Structure (by ref)"))
  (bind (_bblockinghit _binitialoverlap _time _distance _location _impactpoint _normal _impactnormal _physmat _hitactor _hitcomponent _hitbonename) (`GameplayStatics.BreakHitResult` Hit))
  (bind _returnvalue (`KismetMathLibrary.Conv_VectorToRotator` HitNormal))
  (bind _aszombie_bp (cast `/Game/所有蓝图/Zombie/Zombie_BP` Other)
    (:`then`
      (`GameplayStatics.SpawnEmitterAtLocation` "/Game/FXResources/GunImpacts/Particles/P_ImpactBlood.P_ImpactBlood" HitLocation _returnvalue (0.5 0.5 0.5))
      (`GameplayStatics.SpawnEmitterAtLocation` "/Game/FXResources/Effects1/SmokeBuilder/Particles/P_SmokePuff1b.P_SmokePuff1b" HitLocation _returnvalue (0.1 0.1 0.1))
      (if (== _hitbonename "head")
        (`GameplayStatics.ApplyDamage` _aszombie_bp 50.0)
        (else
          (`GameplayStatics.ApplyDamage` _aszombie_bp 20.0)))
      (`GameplayStatics.PlaySoundAtLocation` "/Game/AudioResources/BulletImpact/Body/bullet_impact_body_flesh_01_Cue.bullet_impact_body_flesh_01_Cue" _location (struct) 1.0 1.0 0.0 null null null))
    (:`CastFailed`
      (bind _returnvalue_2 (`GameplayStatics.SpawnDecalAtLocation` "/Game/FXResources/Bullet_Impact_Decal.Bullet_Impact_Decal" (7.0 7.0 7.0) HitLocation _returnvalue 20.0))
      (`DecalComponent.SetFadeScreenSize` _returnvalue_2 0.0)
      (`self.击中物体特效` Hit)))
  (`|ExecutionSequence`
    (:`then_0`
      (`/Engine/EditorBlueprintResources/StandardMacros.IsValid` OtherComp
        (:`Is Valid`
          (if (`SceneComponent.IsSimulatingPhysics` OtherComp "None")
            (`PrimitiveComponent.AddImpulse` OtherComp (* (`self.GetVelocity`) 2.0) "None" false)))))
    (:`then_1`
      (`self.K2_DestroyActor`))))

(fn `UserConstructionScript`)

(fn `击中物体特效`
  (params (Hit :type "HitResult Structure"))
  (bind (_bblockinghit _binitialoverlap _time _distance _location _impactpoint _normal) (`GameplayStatics.BreakHitResult` Hit))
  (bind _returnvalue (`KismetMathLibrary.Conv_VectorToRotator` _normal))
  (bind _outhit (`KismetSystemLibrary.SphereTraceSingle` _impactpoint _impactpoint 10.0 "TraceTypeQuery3"))
  (switch `EPhysicalSurface` (`GameplayStatics.GetSurfaceType` _outhit)
    (:`SurfaceType_Default`
      (`GameplayStatics.SpawnEmitterAtLocation` "/Game/FXResources/GunImpacts1/Particles/P_ImpactDirt.P_ImpactDirt" _impactpoint _returnvalue (0.6 0.6 0.6))
      (`GameplayStatics.PlaySoundAtLocation` "/Game/AudioResources/BulletImpact/Gravel/bullet_impact_gravel_01_Cue.bullet_impact_gravel_01_Cue" _impactpoint (struct) 1.0 1.0 0.0 null null null))
    (:`SurfaceType1`
      (`GameplayStatics.SpawnEmitterAtLocation` "/Game/FXResources/GunImpacts1/Particles/P_ImpactMetal.P_ImpactMetal" _impactpoint _returnvalue (0.6 0.6 0.6))
      (`GameplayStatics.PlaySoundAtLocation` "/Game/AudioResources/BulletImpact/Metal/bullet_impact_metal_heavy_01_Cue.bullet_impact_metal_heavy_01_Cue" _impactpoint (struct) 1.0 1.0 0.0 null null null))
    (:`SurfaceType2`
      (`GameplayStatics.SpawnEmitterAtLocation` "/Game/FXResources/GunImpacts1/Particles/P_ImpactDirt.P_ImpactDirt" _impactpoint _returnvalue (0.6 0.6 0.6))
      (`GameplayStatics.PlaySoundAtLocation` "/Game/AudioResources/BulletImpact/Gravel/bullet_impact_gravel_01_Cue.bullet_impact_gravel_01_Cue" _impactpoint (struct) 1.0 1.0 0.0 null null null))
    (:`SurfaceType3`
      (`GameplayStatics.SpawnEmitterAtLocation` "/Game/FXResources/P_ImpactConcrete.P_ImpactConcrete" _impactpoint _returnvalue (0.6 0.6 0.6))
      (`GameplayStatics.PlaySoundAtLocation` "/Game/AudioResources/BulletImpact/Concrete/bullet_impact_concrete_brick_01_Cue.bullet_impact_concrete_brick_01_Cue" _impactpoint (struct) 1.0 1.0 0.0 null null null))
    (:`SurfaceType4`
      (`GameplayStatics.SpawnEmitterAtLocation` "/Game/FXResources/GunImpacts1/Particles/P_ImpactWood.P_ImpactWood" _impactpoint _returnvalue (0.6 0.6 0.6))
      (`GameplayStatics.PlaySoundAtLocation` "/Game/AudioResources/BulletImpact/Wood/bullet_impact_wood_heavy_01_Cue.bullet_impact_wood_heavy_01_Cue" _impactpoint (struct) 1.0 1.0 0.0 null null null))
    (:`SurfaceType5`
      (`GameplayStatics.SpawnEmitterAtLocation` "/Game/FXResources/GunImpacts1/Particles/P_ImpactRock.P_ImpactRock" _impactpoint _returnvalue (0.6 0.6 0.6))
      (`GameplayStatics.PlaySoundAtLocation` "/Game/AudioResources/BulletImpact/Rock/bullet_impact_rock_01_Cue.bullet_impact_rock_01_Cue" _impactpoint (struct) 1.0 1.0 0.0 null null null))
    (:`SurfaceType6`
      (`GameplayStatics.SpawnEmitterAtLocation` "/Game/FXResources/GunImpacts1/Particles/P_ImpactGrass.P_ImpactGrass" _impactpoint _returnvalue (0.6 0.6 0.6))
      (`GameplayStatics.PlaySoundAtLocation` "/Game/AudioResources/Grass/footstep_grass_run_01_Cue.footstep_grass_run_01_Cue" _impactpoint (struct) 1.0 1.0 0.0 null null null))))